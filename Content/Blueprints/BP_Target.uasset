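; Orbit target that checks whether the player's spawned celestial body stays between a minimum and maximum distance.
; Each tick, CheckWin counts consecutive in-range frames, enables the body's post-process and sets InGoodOrbit at TimerMax, resetting on exit until then.
; UpdateText shows French hints with remaining frames or current distance, delaying out-of-range updates.
; The text turns toward the player's free view once, at BeginPlay.
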(event EventBeginPlay
  (|CallParentFunction)
  (bind _asbp_player (Utilities|Casting|CastToBP_Player (Game|Player|GetPlayerPawn 0)))
  (Variables|Default|SetPlayerPawn _asbp_player)
  (CallFunction|RotateText))

(event Collision|EventActorBeginOverlap
  (params (OtherActor :type Actor%20Object%20Reference)))

(event EventTick
  (params (DeltaSeconds :type Float%20%28single-precision%29))
  (|CallParentFunction DeltaSeconds)
  (CallFunction|CheckWin)
  (Utilities|UpdateText))

(fn ConstructionScript
  (|CallParentFunction)
  (if (Physics|IsSimulatingPhysics (Variables|Default|GetStaticMeshComponent) "None")
    _))

(fn CheckWin
  (bind _playerpawn (Variables|Default|GetPlayerPawn))
  (bind _m_spawned (Variables|/Script/ProjetBachelor.CAPlayerPawn|Getm_Spawned _playerpawn))
  (Utilities|IsValid _m_spawned
    (:Is%20Valid
      (if (not (Variables|Default|GetInGoodOrbit))
        (bind _asbp_celestial_body (Utilities|Casting|CastToBP_CelestialBody _m_spawned))
        (if (CallFunction|VerifyDistance _m_spawned)
          (Variables|/Script/Engine.PostProcessComponent|SetbEnabled (Variables|/Game/Blueprints/BP_CelestialBody.BP_CelestialBody_C|GetPostProcess _asbp_celestial_body) true)
          (Math|Integer|IncrementInt (Variables|Default|GetTimer)
            (:%20%20
              (if (== (Variables|Default|GetTimer) (Variables|Default|GetTimerMax))
                (Variables|Default|SetInGoodOrbit true)
                (Variables|/Script/Engine.PostProcessComponent|SetbEnabled (Variables|/Game/Blueprints/BP_CelestialBody.BP_CelestialBody_C|GetPostProcess _asbp_celestial_body) true))))
          (else
            (Variables|/Script/Engine.PostProcessComponent|SetbEnabled (Variables|/Game/Blueprints/BP_CelestialBody.BP_CelestialBody_C|GetPostProcess _asbp_celestial_body) false)
            (Variables|Default|SetTimer 0)))))))

(fn VerifyDistance
  (params (OtherActor :type Actor%20Object%20Reference))
  (return (Math|Float|InRange(Float) (Transformation|GetDistanceTo OtherActor) (Variables|Default|GetTargetMinDistance) (Variables|Default|GetTargetMaxDistance))))

(fn RotateText
  (Transformation|SetWorldRotation (Variables|Default|GetTextRender) (Math|Rotator|FindLookatRotation (Transformation|GetActorLocation) (Transformation|GetWorldLocation (Variables|/Script/ProjetBachelor.CAPlayerPawn|Getm_FreeView (Variables|Default|GetPlayerPawn)))) false true))

(fn UpdateTextValue
  (bind _playerpawn (Variables|Default|GetPlayerPawn))
  (bind _m_spawned (Variables|/Script/ProjetBachelor.CAPlayerPawn|Getm_Spawned _playerpawn))
  (bind _returnvalue (Transformation|GetDistanceTo _m_spawned))
  (bind _returnvalue_2 (Math|Float|Round _returnvalue))
  (bind _returnvalue_3 (Utilities|String|ToString(Integer) _returnvalue_2))
  (Utilities|IsValid _m_spawned
    (:Is%20Valid
      (if (and (> _returnvalue (Variables|Default|GetTargetMinDistance)) (< _returnvalue (Variables|Default|GetTargetMaxDistance)))
        (Variables|Default|SetTargetHintIndex 0)
        (Rendering|Components|TextRender|SetText (Variables|Default|GetTextRender) (Utilities|Text|ToText(String) (Utilities|String|Append (Utilities|Select :Index (Variables|Default|GetTargetHintIndex) :Option%200 (Utilities|String|MakeLiteralString "Bonne orbite") :Option%201 (Utilities|String|MakeLiteralString "Trop proche") :Option%202 (Utilities|String|MakeLiteralString "Trop loin")) " : " (Utilities|Select :Index (Variables|Default|GetTargetHintIndex) :Option%200 (Utilities|String|ToString(Integer) (- (Variables|Default|GetTimerMax) (Variables|Default|GetTimer))) :Option%201 _returnvalue_3 :Option%202 _returnvalue_3))) :!label _label)
        (elif (< _returnvalue (Variables|Default|GetTargetMinDistance))
          (Variables|Default|SetTargetHintIndex 1)
          (goto _label)
          (elif (> _returnvalue (Variables|Default|GetTargetMaxDistance))
            (Variables|Default|SetTargetHintIndex 2)
            (goto _label)))))))