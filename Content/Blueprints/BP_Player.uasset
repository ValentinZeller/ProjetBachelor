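; BP_Player is the player Blueprint that launches celestial bodies and adds the Player widget to the viewport.
; LaunchingSpeed derives a clamped speed from vertical movement, and IsLaunching checks for charging outside free view.
; Launch replaces the previous BP_CelestialBody with one fired along the actor's forward vector, enables its custom depth, and briefly hides the preview Sphere.
; The EventGraph's charge and launch chains have no triggering events, so they never run.
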(event EventBeginPlay
  ;[1 1 1] Création de l'interface utilisateur
  (bind _returnvalue (UserInterface|CreateWidget "/Game/UI/Player.Player_C"))
  (UserInterface|Viewport|AddtoViewport _returnvalue 0))

(event Collision|EventActorBeginOverlap
  (params (OtherActor :type Actor%20Object%20Reference)))

(event EventTick
  (params (DeltaSeconds :type Float%20%28single-precision%29)))

(event Input|ActionEvents|InputActionLaunch
  (params (Key :type Key%20Structure :default "None"))
  ;[0.3094 0.3618 1] Lancement de corps céleste
)

(fn ConstructionScript
  (Variables|Default|Setm_Sphere (Variables|Default|GetSphere)))

(fn LaunchingSpeed
  (bind _output_get (Variables|Default|Setm_fInitialSpeed (Math|Float|Clamp(Float) (* (Input|AxisValues|GetVerticalMovement) (Math|Float|MakeLiteralFloat -1e+01)) 0.0 (Variables|Default|GetMaxSpeed))))
  (return _output_get))