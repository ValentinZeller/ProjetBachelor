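; BP_SoloGameMode is a game mode that handles level completion and progression in solo play.
; Every tick it looks up the BP_Target actor and checks its InGoodOrbit flag.
; When that flag is set, a DoOnce plays a sound, waits, then opens the level following the current one in the LevelsName array, or StartMenu after the last.
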(event EventBeginPlay)

(event EventTick
  (params (DeltaSeconds :type Float%20%28single-precision%29))
  (bind _levelsname (Variables|Default|GetLevelsName))
  (bind _returnvalue (Actor|GetActorOfClass "/Game/Blueprints/BP_Target.BP_Target_C"))
  (if (Variables|/Game/Blueprints/BP_Target.BP_Target_C|GetInGoodOrbit _returnvalue)
    (Utilities|FlowControl|DoOnce false
      (:Completed
        (Audio|PlaySound2D "/Game/Musics/clip_04_intro-448.clip_04_intro-448" 1.0 1.0 0.0 0 0)
        (Utilities|FlowControl|Delay 7.0)
        (bind _returnvalue_2 (Game|GetCurrentLevelName true))
        (if (== (Utilities|Array|LastIndex _levelsname) (Utilities|Array|FindItem _levelsname (Utilities|String|StringToName _returnvalue_2)))
          (Game|OpenLevel(byName) "StartMenu")
          (else
            (bind _result (Math|Integer|IncrementInt (Utilities|Array|FindItem _levelsname (Utilities|String|StringToName _returnvalue_2)))
              (:%20%20
                (Game|OpenLevel(byName) (Utilities|Array|Get(acopy) _levelsname _result))))))))))

(fn ConstructionScript)