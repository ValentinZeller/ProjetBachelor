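; Game mode for a local two-player, turn-based match in which both BP_Player pawns share one player controller.
; BeginPlay spawns the second player, hidden and with its own planet material, then caches both pawns.
; Tick polls the current player's HasSpawned flag to swap visibility, possession and widget via a boolean index, counting rounds.
; After MaxTurn, it unpossesses, clears the UI and shows an end widget after a delay.
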(event EventBeginPlay
  (CallFunction|CreatePlayer)
  (bind _returnvalue (Actor|GetActorOfClass "/Game/Blueprints/BP_Player.BP_Player_C"))
  (Variables|/Script/ProjetBachelor.CAPlayerPawn|SetbDestroySpawned _returnvalue false)
  (bind _outactors (Actor|GetAllActorsOfClass "/Game/Blueprints/BP_Player.BP_Player_C"))
  (Variables|Default|SetPlayers _outactors))

(event EventTick
  (params (DeltaSeconds :type Float%20%28single-precision%29))
  (bind _currentplayer (CallFunction|GetPlayers))
  (bind _returnvalue (Game|GetPlayerController 0))
  (bind _output_get (Variables|Default|SetIsNotFinished (< (Variables|Default|GetCurrentTurn) (Variables|Default|GetMaxTurn))))
  (if _output_get
    (if (Variables|/Script/ProjetBachelor.CAPlayerPawn|GetbHasSpawned _currentplayer)
      (Variables|/Script/ProjetBachelor.CAPlayerPawn|SetbHasSpawned _currentplayer false)
      (CallFunction|SwitchPlayer)
      (if (== (Utilities|Array|Get(acopy) (Variables|Default|GetPlayers)) _currentplayer)
        (Math|Integer|IncrementInt (Variables|Default|GetCurrentTurn))))
    (else
      (Utilities|FlowControl|DoOnce false
        (:Completed
          (Pawn|UnPossess _returnvalue)
          (Rendering|SetVisibility (Variables|/Game/Blueprints/BP_Player.BP_Player_C|GetSphere _currentplayer) false false)
          (Viewport|RemoveAllWidgets)
          (Utilities|FlowControl|Delay (Variables|Default|GetDelayBeforeEnd))
          (bind _returnvalue_2 (UserInterface|CreateWidget "/Game/UI/MultiplayerEnd.MultiplayerEnd_C"))
          (UserInterface|Viewport|AddtoViewport _returnvalue_2 0)
          (Input|SetInputModeGameandUI _returnvalue _returnvalue_2 "DoNotLock" false)
          (Variables|/Script/Engine.PlayerController|SetbShowMouseCursor _returnvalue true))))))

(fn ConstructionScript)

(fn SwitchPlayer
  (bind _returnvalue (Game|GetPlayerController 0))
  (bind (_currentplayer _otherindex _otherplayer) (CallFunction|GetPlayers))
  (Rendering|SetVisibility (Variables|/Game/Blueprints/BP_Player.BP_Player_C|GetSphere _currentplayer) false true)
  (Rendering|SetVisibility (Variables|/Game/Blueprints/BP_Player.BP_Player_C|GetSphere _otherplayer) true true)
  (Pawn|UnPossess _returnvalue)
  (Pawn|Possess _returnvalue _otherplayer)
  (Viewport|RemoveAllWidgets)
  (UserInterface|Viewport|AddtoViewport (Variables|/Game/Blueprints/BP_Player.BP_Player_C|GetPlayerWidget _otherplayer) 0)
  (Variables|Default|SetCurrentPlayerIndex _otherindex))

(fn GetPlayers
  (bind _currentplayerindex (Variables|Default|GetCurrentPlayerIndex))
  (bind _players (Variables|Default|GetPlayers))
  (bind _returnvalue (not _currentplayerindex))
  (return (Utilities|Array|Get(acopy) _players (Math|Conversions|ToInteger(Boolean) _currentplayerindex)) _returnvalue (Utilities|Array|Get(acopy) _players (Math|Conversions|ToInteger(Boolean) _returnvalue))))

(fn CreatePlayer
  (bind _returnvalue (Actor|GetActorOfClass "/Script/Engine.PlayerStart"))
  (bind _returnvalue_2 (Game|SpawnActorfromClass "/Game/Blueprints/BP_Player.BP_Player_C" (Transformation|GetActorTransform _returnvalue) "Undefined" 0 0))
  (Utilities|FlowControl|Sequence
    (:then_0
      (Variables|/Script/ProjetBachelor.CAPlayerPawn|SetbDestroySpawned _returnvalue_2 false)
      (Variables|/Script/ProjetBachelor.CAPlayerPawn|SetSpawnedMaterial _returnvalue_2 "/Game/Materials/M_Planet_Player2.M_Planet_Player2"))
    (:then_1
      (Rendering|Material|SetMaterial (Variables|/Game/Blueprints/BP_Player.BP_Player_C|GetSphere _returnvalue_2) 0 "/Game/Materials/M_Planet_Player2.M_Planet_Player2")
      (Rendering|SetVisibility (Variables|/Game/Blueprints/BP_Player.BP_Player_C|GetSphere _returnvalue_2) false true))))