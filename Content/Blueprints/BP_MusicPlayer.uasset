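; BP_MusicPlayer is a music player that plays random tracks from a Playlist array through its Audio component.
; On BeginPlay it assigns a random Playlist entry to Audio and starts playback.
; Each OnAudioFinished event repeats the pick and play, so music continues back to back, and the same track can play twice in a row.
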(event OnAudioFinished(Audio)
  (bind _audio (Variables|Default|GetAudio))
  (Audio|Components|Audio|SetSound _audio (.OutItem (Utilities|Array|Random (Variables|Default|GetPlaylist))))
  (Audio|Components|Audio|Play _audio 0.0))

(event EventBeginPlay
  (bind _audio (Variables|Default|GetAudio))
  (Audio|Components|Audio|SetSound _audio (.OutItem (Utilities|Array|Random (Variables|Default|GetPlaylist))))
  (Audio|Components|Audio|Play _audio 0.0))

(event EventTick
  (params (DeltaSeconds :type Float%20%28single-precision%29)))

(fn ConstructionScript)