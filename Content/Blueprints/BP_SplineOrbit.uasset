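; BP_SplineOrbit draws a circular orbit ring of static meshes, sized from BP_Target's TargetMaxDistance.
; The construction script takes a tenth of that distance as radius, then builds four local spline points with hand-set tangents approximating a circle.
; CreateMesh closes the loop and adds non-simulating mesh components at SplineSpacing intervals, using world-space spline transforms with manual attachment.
; All work happens at construction, with no active runtime logic.
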(event EventBeginPlay)

(event Collision|EventActorBeginOverlap
  (params (OtherActor :type Actor%20Object%20Reference)))

(event EventTick
  (params (DeltaSeconds :type Float%20%28single-precision%29)))

(fn ConstructionScript
  (bind _returnvalue (Actor|GetActorOfClass "/Game/Blueprints/BP_Target.BP_Target_C"))
  (Variables|Default|SetSplineRadius (/ (Variables|/Game/Blueprints/BP_Target.BP_Target_C|GetTargetMaxDistance _returnvalue) (Math|Float|MakeLiteralFloat 1e+01)))
  (CallFunction|CreatePoints)
  (for _index (range 0 (Spline|GetNumberOfSplinePoints (Variables|Default|GetSpline)))
    (Variables|Default|SetSplineNum _index)
    (CallFunction|CreateTangents))
  (CallFunction|CreateMesh))

(fn CreatePoints
  (bind _splineradius (Variables|Default|GetSplineRadius))
  (bind _spline (Variables|Default|GetSpline))
  (bind _spline_2 (Variables|Default|GetSpline))
  (bind _returnvalue (* _splineradius -1.0))
  (Spline|ClearSplinePoints _spline true)
  (Spline|AddSplinePoint _spline (Math|Vector|MakeVector _splineradius 0.0 0.0) "Local" true)
  (Spline|AddSplinePoint _spline (Math|Vector|MakeVector 0.0 _splineradius 0.0) "Local" true)
  (Spline|AddSplinePoint _spline_2 (Math|Vector|MakeVector _returnvalue 0.0 0.0) "Local" true)
  (Spline|AddSplinePoint _spline_2 (Math|Vector|MakeVector 0.0 _returnvalue 0.0) "Local" true))

(fn CreateTangents
  (bind _splinenum (Variables|Default|GetSplineNum))
  (bind _splinenum_2 (Variables|Default|GetSplineNum))
  (bind _splinenum_3 (Variables|Default|GetSplineNum))
  (bind _splinenum_4 (Variables|Default|GetSplineNum))
  (if (== _splinenum_2 0)
    (Spline|SetTangentatSplinePoint (Variables|Default|GetSpline) _splinenum_2 (Math|Vector|MakeVector 0.0 (* (* (Variables|Default|GetSplineRadius) 1.5) 1.0) 0.0) "Local" true)
    (elif (== _splinenum_3 1)
      (Spline|SetTangentatSplinePoint (Variables|Default|GetSpline) _splinenum_3 (Math|Vector|MakeVector (* (* (Variables|Default|GetSplineRadius) 1.5) -1.0) 0.0 0.0) "Local" true)
      (elif (== _splinenum_4 2)
        (Spline|SetTangentatSplinePoint (Variables|Default|GetSpline) _splinenum_4 (Math|Vector|MakeVector 0.0 (* (* (Variables|Default|GetSplineRadius) 1.5) -1.0) 0.0) "Local" true)
        (elif (== _splinenum 3)
          (Spline|SetTangentatSplinePoint (Variables|Default|GetSpline) _splinenum (Math|Vector|MakeVector (* (* (Variables|Default|GetSplineRadius) 1.5) 1.0) 0.0 0.0) "Local" true))))))

(fn CreateMesh
  (bind _spline (Variables|Default|GetSpline))
  (bind _splinespacing (Variables|Default|GetSplineSpacing))
  (Spline|SetClosedLoop _spline true true)
  (for _index (range 0 (.ReturnValue (Math|Float|Division(WholeandRemainder) (Spline|GetSplineLength _spline) _splinespacing)))
    (bind _returnvalue (AddComponent|AddStaticMeshComponent true (Math|Transform|MakeTransform (Spline|GetLocationatDistanceAlongSpline (Variables|Default|GetSpline) (* _index _splinespacing) "World") (Spline|GetRotationatDistanceAlongSpline (Variables|Default|GetSpline) (* _index _splinespacing) "World"))))
    (Components|StaticMesh|SetStaticMesh _returnvalue (Variables|Default|GetMesh))
    (Rendering|Material|SetMaterial _returnvalue 0 (Variables|Default|GetMaterial))
    (Physics|SetSimulatePhysics _returnvalue false)))