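; Multiplayer sun actor that labels which player ("Joueur" plus a number) is winning, based on the celestial body nearest to it.
; While the multiplayer game mode is unfinished, Tick scans all BP_CelestialBody actors except itself and tracks the closest.
; The text updates from that body's first tag compared with Player1Name.
; At BeginPlay, the TextRender is rotated once toward the player pawn's MFreeView.
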(event EventBeginPlay
  (|CallParentFunction)
  (bind _asbp_player (Utilities|Casting|CastToBP_Player (Game|Player|GetPlayerPawn 0)))
  (Variables|Default|SetPlayerPawn _asbp_player)
  (CallFunction|RotateText))

(event Collision|EventActorBeginOverlap
  (params (OtherActor :type Actor%20Object%20Reference)))

(event EventTick
  (params (DeltaSeconds :type Float%20%28single-precision%29))
  (|CallParentFunction DeltaSeconds)
  (bind _asbp_multiplayer_game_mode (Utilities|Casting|CastToBP_MultiplayerGameMode (Game|GetGameMode)))
  (if (Variables|/Game/Blueprints/BP_MultiplayerGameMode.BP_MultiplayerGameMode_C|GetIsNotFinished _asbp_multiplayer_game_mode)
    (CallFunction|GetNearest)))

(fn ConstructionScript
  (|CallParentFunction))

(fn RotateText
  (Transformation|SetWorldRotation (Variables|Default|GetTextRender) (Math|Rotator|FindLookatRotation (Transformation|GetActorLocation) (Transformation|GetWorldLocation (Variables|/Script/ProjetBachelor.CAPlayerPawn|Getm_FreeView (Variables|Default|GetPlayerPawn)))) false true))

(fn GetNearest
  (bind _outactors (Actor|GetAllActorsOfClass "/Game/Blueprints/BP_CelestialBody.BP_CelestialBody_C"))
  (for _array_element _outactors
    (Utilities|NotSameName _array_element
      (:Not%20Same
        (Utilities|IsValid (Variables|Default|GetNearest)
          (:Is%20Valid
            (if (<= (Transformation|GetDistanceTo _array_element) (Transformation|GetDistanceTo (Variables|Default|GetNearest)))
              (Variables|Default|SetNearest _array_element)
              (CallFunction|UpdateText)))
          (:Is%20Not%20Valid
            (Variables|Default|SetNearest _array_element)))))))

(fn UpdateText
  (bind _output_get (Variables|Default|SetPlayerWinning (Utilities|Name|Equal(Name) (Utilities|Array|Get(acopy) (Variables|/Script/Engine.Actor|GetTags (Variables|Default|GetNearest))) (Variables|Default|GetPlayer1Name))))
  (bind _result (Math|Integer|IncrementInt (Math|Conversions|ToInteger(Boolean) _output_get))
    (:%20%20
      (Rendering|Components|TextRender|SetText (Variables|Default|GetTextRender) (Utilities|Text|ToText(String) (Utilities|String|Append "Joueur " (Utilities|String|ToString(Integer) _result)))))))