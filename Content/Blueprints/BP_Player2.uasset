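; BP_Player2 is a player pawn that aims and launches a BP_CelestialBody toward a distance band around a "Target" body.
; Yaw/pitch input aims, or flies a toggleable free camera.
; Holding left mouse locks aim; release converts current vertical axis input into clamped speed and spawns the body, replacing the previous one.
; Tick runs CheckWin, which only prints the distance when the spawned body is inside the band.
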(event EventBeginPlay
  (bind _returnvalue (UserInterface|CreateWidget "/Game/UI/Player.Player_C"))
  (UserInterface|Viewport|AddtoViewport _returnvalue 0))

(event Collision|EventActorBeginOverlap
  (params (OtherActor :type Actor%20Object%20Reference)))

(event EventTick
  (params (DeltaSeconds :type Float%20%28single-precision%29))
  (CallFunction|CheckWin (Variables|Default|GetSpawned))
  (if (Variables|Default|GetIsCharging)
    (CallFunction|LaunchingSpeed)))

(event Input|ActionEvents|InputActionChangeCameraView
  (params (Key :type Key%20Structure :default "None"))
  (:Pressed
    (if (Variables|Default|GetisFreeView)
      (Variables|Default|SetisFreeView false)
      (Transformation|ResetRelativeTransform (Variables|Default|GetfreeView))
      (Components|Activation|SetActive (Variables|Default|GetfreeView) false false)
      (Components|Activation|SetActive (Variables|Default|GetCamera) true false)
      (else
        (Variables|Default|SetisFreeView true)
        (Variables|Default|SetIsCharging false)
        (Components|Activation|SetActive (Variables|Default|GetCamera) false false)
        (Components|Activation|SetActive (Variables|Default|GetfreeView) true false)))))

(event Input|AxisEvents|InputAxisHorizontalMovement
  (params (AxisValue :type Float%20%28single-precision%29))
  (if (Math|Boolean|NORBoolean (Variables|Default|GetIsCharging) (Variables|Default|GetisFreeView))
    (Pawn|Input|AddControllerYawInput AxisValue)
    (elif (Variables|Default|GetisFreeView)
      (Transformation|AddLocalRotation (Variables|Default|GetfreeView) (Math|Rotator|MakeRotator 0.0 0.0 AxisValue) false false))))

(event Input|AxisEvents|InputAxisVerticalMovement
  (params (AxisValue :type Float%20%28single-precision%29))
  (if (Math|Boolean|NORBoolean (Variables|Default|GetIsCharging) false)
    (Pawn|Input|AddControllerPitchInput AxisValue)
    (elif (Variables|Default|GetisFreeView)
      (Transformation|AddLocalRotation (Variables|Default|GetfreeView) (Math|Rotator|MakeRotator 0.0 (* AxisValue -1.0) 0.0) false false))))

(event Input|AxisEvents|InputAxisMoveForwardBackward
  (params (AxisValue :type Float%20%28single-precision%29))
  (if (Variables|Default|GetisFreeView)
    (Transformation|AddLocalOffset (Variables|Default|GetfreeView) (Math|Vector|MakeVector (* AxisValue (Variables|Default|GetMovementMultiplier)) 0.0 0.0) false false)))

(event Input|AxisEvents|InputAxisMoveRightLeft
  (params (AxisValue :type Float%20%28single-precision%29))
  (if (Variables|Default|GetisFreeView)
    (Transformation|AddLocalOffset (Variables|Default|GetfreeView) (Math|Vector|MakeVector 0.0 (* AxisValue (Variables|Default|GetMovementMultiplier)) 0.0) false false)))

(event Input|MouseEvents|LeftMouseButton
  (params (Key :type Key%20Structure :default "None"))
  (:Pressed
    (Variables|Default|SetIsCharging true))
  (:Released
    (Utilities|IsLaunching
      (:True
        (Variables|Default|SetIsCharging false)
        (bind _speed (CallFunction|LaunchingSpeed))
        (Utilities|Launch _speed)))))

(fn ConstructionScript)

(fn LaunchingSpeed
  (bind _output_get (Variables|Default|SetInitialSpeed (Math|Float|Clamp(Float) (* (Input|AxisValues|GetVerticalMovement) (Math|Float|MakeLiteralFloat -1e+01)) 0.0 (Variables|Default|GetMaxSpeed))))
  (return _output_get))

(fn CheckWin
  (params (OtherActor :type Actor%20Object%20Reference))
  (bind _targetdistance (Variables|Default|GetTargetDistance))
  (bind _outactors (Actor|GetAllActorswithTag "Target"))
  (bind _asbp_celestial_body (Utilities|Casting|CastToBP_CelestialBody (Utilities|Array|Get(acopy) _outactors)))
  (if (Math|Float|InRange(Float) (Transformation|GetDistanceTo _asbp_celestial_body OtherActor) (- _targetdistance 1e+02) _targetdistance)
    (Development|PrintString (Utilities|String|ToString(Float) (Transformation|GetDistanceTo _asbp_celestial_body OtherActor)))))