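; BP_CelestialBody is a space body actor that spins its static mesh by a fixed local rotation every tick, independent of delta time.
; The construction script enables physics simulation on the mesh.
; Helper functions provide gravity-style inputs: scaled body mass, a constant divided by unsquared distance to another space actor, and an unnormalized direction between component locations.
; None of these helpers are called within this Blueprint.
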(event EventTick
  (params (DeltaSeconds :type Float%20%28single-precision%29))
  (Transformation|AddLocalRotation (Variables|Default|GetStaticMeshComponent) "0,5.000000, 0" false false))

(event EventBeginPlay)

(fn ConstructionScript
  (bind _staticmeshcomponent (Variables|Default|GetStaticMeshComponent))
  (if (not (Physics|IsSimulatingPhysics _staticmeshcomponent "None"))
    (Physics|SetSimulatePhysics _staticmeshcomponent true)))

(fn GetBodyMass
  (params (Space%20Primitive%20Component :type Primitive%20Component%20Object%20Reference))
  (return (* (Class|PrimitiveComponent|GetMassScale Space%20Primitive%20Component "None") (Physics|GetMass Space%20Primitive%20Component))))

(fn GetDistanceBetweenBodies
  (if (!= self (Variables|Default|GetSpaceActor))
    (return (/ (Variables|Default|GetConstant) (Transformation|GetDistanceTo self (Variables|Default|GetSpaceActor))))))

(fn GetDirection
  (return (- (Transformation|GetWorldLocation (Actor|GetComponentbyClass self "/Script/Engine.PrimitiveComponent")) (Transformation|GetWorldLocation (Variables|Default|GetSpacePrimitiveComponent)))))